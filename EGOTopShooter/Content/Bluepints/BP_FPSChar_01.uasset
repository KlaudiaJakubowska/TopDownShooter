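; BP_FPSChar_01 is a player character with an assault rifle particle effect, looping-style fire audio control and a HUD created at BeginPlay.
; Fire input toggles the effect and starts or stops the weapon sound, while axis inputs move along the player controller's forward and right vectors.
; Each Tick, mouse velocity beyond a dead zone sets a target yaw from its direction, interpolated into control rotation.
; AnyDamage sets Dead only when Health minus Damage equals zero.
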(event `InputAction|Fire`
  (params (Key :type "Key Structure"))
  (:`Pressed`
    (`ActorComponent.Activate` (`self.P_AssaultRifle_MF`) false)
    (bind _returnvalue (`GameplayStatics.SpawnSound2D` "/Game/Sounds/Weapon_AssaultRifle/Stereo/SC_WeaponFired_01.SC_WeaponFired_01" 1.0 1.0 0.0 null))
    (set `self.Weapon sound` _returnvalue))
  (:`Released`
    (`ActorComponent.Deactivate` (`self.P_AssaultRifle_MF`))
    (`AudioComponent.Stop` (`self.Weapon sound`))
    (`GameplayStatics.SpawnSound2D` null 1.0 1.0 0.0 null)))

(event `self.ReceiveBeginPlay`
  (bind _returnvalue (`|CreateWidget` "/Game/UI/W_PlayerHUD_01.W_PlayerHUD_01_C" null self))
  (`UserWidget.AddToViewport` _returnvalue 0))

(event `self.ReceiveTick`
  (params (DeltaSeconds :type "Float (single-precision)"))
  (`self.CharacterRotate`))

(event `InputAxis|MoveForewardBack`
  (params (AxisValue :type "Float (single-precision)"))
  (`self.AddMovementInput` (`self.GetActorForwardVector` (`GameplayStatics.GetPlayerController` 0)) AxisValue))

(event `self.ReceiveAnyDamage`
  (params (Damage :type "Float (single-precision)") (DamageType :type "DamageType Object Reference") (InstigatedBy :type "Controller Object Reference") (DamageCauser :type "Actor Object Reference"))
  (set `self.Dead` (== (- (`self.Health`) Damage) 0.0)))

(event `InputAxis|MoveLeftRight`
  (params (AxisValue :type "Float (single-precision)"))
  (`self.AddMovementInput` (`self.GetActorRightVector` (`GameplayStatics.GetPlayerController` 0)) AxisValue))

(fn `CharacterRotate`
  (bind _returnvalue (`GameplayStatics.GetPlayerController` 0))
  (bind (_returnvalue_x _returnvalue_y) (`KismetMathLibrary.BreakVector2D` (`self.MouseVelocity`)))
  (if (`self.IsMouseDeadZone`)
    (`Controller.SetControlRotation` _returnvalue (`KismetMathLibrary.RInterpTo` (`Controller.GetControlRotation` _returnvalue) (`KismetMathLibrary.MakeRotator` 0.0 0.0 (`KismetMathLibrary.DegAtan2` _returnvalue_x _returnvalue_y)) (`GameplayStatics.GetWorldDeltaSeconds`) (`self.Interp Speed`)))))

(fn `IsMouseDeadZone`
  (returns (ReturnValue :type Boolean))
  (return (> (`KismetMathLibrary.VSize2D` (`self.MouseVelocity`)) (`self.DeadZone`))))

(fn `MouseVelocity`
  (returns (ReturnValue :type "Vector2D Structure"))
  (bind (_deltax _deltay) (`PlayerController.GetInputMouseDelta` (`GameplayStatics.GetPlayerController` 0)))
  (return (/ (`KismetMathLibrary.MakeVector2D` _deltax _deltay) (`GameplayStatics.GetWorldDeltaSeconds`))))

(fn `UserConstructionScript`)